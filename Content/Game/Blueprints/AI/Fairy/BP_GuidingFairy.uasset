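; BP_GuidingFairy is a fairy companion that trails the player and delivers dialogue through a WBP_Fairy widget.
; Each tick it eases toward a point diagonally front-right of the player pawn and turns the widget to face the follow camera.
; PlayDialogue hands a dialogue number to the widget, while SkipDialogue fires that dialogue's event and finishes.
; Finishing deactivates the PProjectile component, hides the widget, then destroys the fairy after a short delay.
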(event Custom|PlayDialogue
  (params (DialogueNum :type Integer))
  (bind _aswbp_fairy (Utilities|Casting|CastToWBP_Fairy (UserInterface|GetWidget (Variables|Default|GetWidget))))
  (Default|RunDialogue _aswbp_fairy DialogueNum self)
  (Variables|Default|SetRunningDialogue DialogueNum))

(event Custom|DialogueFinished
  (Components|Activation|Deactivate (Variables|Default|GetP_Projectile))
  (Rendering|SetVisibility (Variables|Default|GetWidget) false false)
  (Utilities|FlowControl|Delay 2.0)
  (Actor|DestroyActor))

(event Custom|SkipDialogue
  (bind _aswbp_fairy (Utilities|Casting|CastToWBP_Fairy (UserInterface|GetWidget (Variables|Default|GetWidget))))
  (Default|RunDialogueEvent _aswbp_fairy (Variables|Default|GetRunningDialogue))
  (CallFunction|DialogueFinished))

(event EventBeginPlay
  (Rendering|SetVisibility (Variables|Default|GetWidget) true false))

(event EventTick
  (params (DeltaSeconds :type Float%20%28single-precision%29))
  (bind _returnvalue (Game|Player|GetPlayerPawn 0))
  (Transformation|SetActorLocation (Math|Interpolation|VInterpTo (Transformation|GetActorLocation) (+ (Transformation|GetActorLocation _returnvalue) (Math|Vector|Lerp(Vector) (* (Transformation|GetActorRightVector _returnvalue) 2e+02) (* (Transformation|GetActorForwardVector _returnvalue) 2e+02) 0.5)) DeltaSeconds 2.0) false false)
  (bind _asbp_third_person_character (Utilities|Casting|CastToBP_ThirdPersonCharacter (Game|Player|GetPlayerPawn 0)))
  (Transformation|SetWorldRotation (Variables|Default|GetWidget) (Math|Rotator|FindLookatRotation (Transformation|GetActorLocation) (Transformation|GetWorldLocation (Variables|/Game/ThirdPerson/Blueprints/BP_ThirdPersonCharacter.BP_ThirdPersonCharacter_C|GetFollowCamera _asbp_third_person_character))) false false))

(fn ConstructionScript)