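; Light golem boss that always faces the player and, after an opening expanding blast, runs a looping random attack AI.
; Each cycle favors repositioning near a point ahead of the player over the expanding blast, laser or spread projectile barrage, each a latent macro spawning its attack actor.
; Damage feeds BPACHealthSystem; death is checked between actions, then plays stun animations and an energy effect, notifies BP_World_Unlock_Manager and destroys the golem.
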(event Custom|StartAI
  (switch int (Math|Random|RandomIntegerinRange 0 6) :!label _label
    (:Default
      _)
    (:0
      (Utilities|MoveAI :!label _label_2
        (:On%20Success
          _)))
    (:1
      (Utilities|ExpandingBlastAttack))
    (:2
      (Utilities|LazarAttack))
    (:3
      (Utilities|ProjectileAttack))
    (:4
      (goto _label_2))
    (:5
      (goto _label_2))
    (:6
      (goto _label_2)))
  (Utilities|FlowControl|Delay 1.0)
  (if (Variables|Default|GetisDead)
    (Components|Animation|PlayAnimation (Variables|Default|GetGolemMain) "/Game/Ancient_Golem/Animation/Animations/Gol_Stun_Start.Gol_Stun_Start" false)
    (Utilities|FlowControl|Delay 1.15)
    (Components|Animation|PlayAnimation (Variables|Default|GetGolemMain) "/Game/Ancient_Golem/Animation/Animations/Gol_Stun_Loop.Gol_Stun_Loop" true)
    (Utilities|FlowControl|Delay 2.0)
    (bind _returnvalue (Niagara|SpawnSystematLocation "/Game/MsvFx_Niagara_SlashFx_Pack/Prefabs/P_Spawn_Energy_Light.P_Spawn_Energy_Light" (- (Transformation|GetWorldLocation (Variables|Default|GetGolemMain)) 1e+02) "0, 0, 0" "7.000000,7.000000,7.000000"))
    (bind _returnvalue_2 (Actor|GetActorOfClass "/Game/Game/Blueprints/World/BP_World_Unlock_Manager.BP_World_Unlock_Manager_C"))
    (Default|CallLightDefeated _returnvalue_2)
    (Utilities|FlowControl|Delay 3.0)
    (Components|Activation|Deactivate _returnvalue)
    (Actor|DestroyActor)
    (else
      (goto _label))))

(event Custom|PlayStartSequence
  (Utilities|ExpandingBlastAttack)
  (Utilities|FlowControl|Delay 1.0)
  (CallFunction|StartAI))

(event Game|Damage|EventAnyDamage
  (params (Damage :type Float%20%28single-precision%29) (DamageType :type Damage%20Type%20Object%20Reference) (InstigatedBy :type Controller%20Object%20Reference) (DamageCauser :type Actor%20Object%20Reference))
  ;[0.04688 0.04688 0.04688 0.88] Take Damage
  (bind _isdead_ (Default|DecreaseHealth (Variables|Default|GetBPAC_HealthSystem) Damage))
  (Variables|Default|SetisDead _isdead_))

(event EventTick
  (params (DeltaSeconds :type Float%20%28single-precision%29))
  (Transformation|SetActorRotation (Math|Rotator|FindLookatRotation (Transformation|GetActorLocation) (Transformation|GetActorLocation (Game|GetPlayerCharacter 0)))))

(fn ConstructionScript
  (Transformation|AttachComponentToComponent (Variables|Default|GetGolemInterior) (Variables|Default|GetGolemMain) "spine_03Socket" "KeepRelative" "KeepRelative" "KeepRelative" true)
  (Transformation|AttachComponentToComponent (Variables|Default|GetGolemHeadRing) (Variables|Default|GetGolemMain) "headSocket" "KeepRelative" "KeepRelative" "KeepRelative" true))