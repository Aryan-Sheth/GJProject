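; BP_LightLazer is a timed multi-beam laser hazard that telegraphs its beams before firing and destroys itself afterward.
; The warning phase shows four cylinders with the four hit boxes' collision disabled.
; After a short delay, the attack phase hides the cylinders, enables collision and spawns a P_Laser effect along each EndPos direction.
; Box overlaps only print a debug hit message; no damage is applied.
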(event OnComponentBeginOverlap(Box4)
  (params (OverlappedComponent :type Primitive%20Component%20Object%20Reference) (OtherActor :type Actor%20Object%20Reference) (OtherComp :type Primitive%20Component%20Object%20Reference) (OtherBodyIndex :type Integer) (bFromSweep :type Boolean) (SweepResult :type Hit%20Result%20Structure%20%28by%20ref%29))
  (Development|PrintString "LazerHit"))

(event OnComponentBeginOverlap(Box9)
  (params (OverlappedComponent :type Primitive%20Component%20Object%20Reference) (OtherActor :type Actor%20Object%20Reference) (OtherComp :type Primitive%20Component%20Object%20Reference) (OtherBodyIndex :type Integer) (bFromSweep :type Boolean) (SweepResult :type Hit%20Result%20Structure%20%28by%20ref%29))
  (Development|PrintString "LazerHit"))

(event OnComponentBeginOverlap(Box5)
  (params (OverlappedComponent :type Primitive%20Component%20Object%20Reference) (OtherActor :type Actor%20Object%20Reference) (OtherComp :type Primitive%20Component%20Object%20Reference) (OtherBodyIndex :type Integer) (bFromSweep :type Boolean) (SweepResult :type Hit%20Result%20Structure%20%28by%20ref%29))
  (Development|PrintString "LazerHit"))

(event OnComponentBeginOverlap(Box10)
  (params (OverlappedComponent :type Primitive%20Component%20Object%20Reference) (OtherActor :type Actor%20Object%20Reference) (OtherComp :type Primitive%20Component%20Object%20Reference) (OtherBodyIndex :type Integer) (bFromSweep :type Boolean) (SweepResult :type Hit%20Result%20Structure%20%28by%20ref%29))
  (Development|PrintString "LazerHit"))

(event EventBeginPlay
  (CallFunction|InitializeWarningPhase)
  (Utilities|FlowControl|Delay 1.5)
  (CallFunction|InitializeAttackPhase)
  (for _array_element (Variables|Default|GetEndPos)
    (bind _returnvalue (Niagara|SpawnSystematLocation "/Game/Lightning_Electricity_Pack/Particles/P_Laser.P_Laser" (Transformation|GetActorLocation)))
    (Niagara|SetNiagaraVariable(Vector3) _returnvalue "EndPosi" (+ (Transformation|GetActorLocation) (* _array_element 5e+03))))
  (Utilities|FlowControl|Delay 5.0)
  (Actor|DestroyActor))

(fn ConstructionScript)

(fn InitializeWarningPhase
  (for _array_element (Utilities|Array|MakeArray (Variables|Default|GetBox5) (Variables|Default|GetBox9) (Variables|Default|GetBox4) (Variables|Default|GetBox10))
    (Collision|SetCollisionEnabled _array_element "NoCollision"))
  (for _array_element_2 (Utilities|Array|MakeArray (Variables|Default|GetCylinder1) (Variables|Default|GetCylinder2) (Variables|Default|GetCylinder3) (Variables|Default|GetCylinder))
    (Rendering|SetVisibility _array_element_2 true false)))

(fn InitializeAttackPhase
  (for _array_element (Utilities|Array|MakeArray (Variables|Default|GetBox5) (Variables|Default|GetBox9) (Variables|Default|GetBox4) (Variables|Default|GetBox10))
    (Collision|SetCollisionEnabled _array_element "QueryAndPhysics"))
  (for _array_element_2 (Utilities|Array|MakeArray (Variables|Default|GetCylinder1) (Variables|Default|GetCylinder2) (Variables|Default|GetCylinder3) (Variables|Default|GetCylinder))
    (Rendering|SetVisibility _array_element_2 false false)))