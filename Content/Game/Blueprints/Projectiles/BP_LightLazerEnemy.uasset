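; Enemy laser attack actor that telegraphs with warning cylinders, then fires damaging beams before destroying itself.
; After a short delay, it hides the cylinders, enables four box hitboxes and spawns a Niagara laser along each EndPos direction.
; Box overlaps start a looping timer that repeatedly damages the overlapping actor until overlap ends, with all boxes sharing one timer handle.
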(event OnComponentEndOverlap(Box4)
  (params (OverlappedComponent :type Primitive%20Component%20Object%20Reference) (OtherActor :type Actor%20Object%20Reference) (OtherComp :type Primitive%20Component%20Object%20Reference) (OtherBodyIndex :type Integer))
  (CallFunction|EndDamage))

(event OnComponentEndOverlap(Box9)
  (params (OverlappedComponent :type Primitive%20Component%20Object%20Reference) (OtherActor :type Actor%20Object%20Reference) (OtherComp :type Primitive%20Component%20Object%20Reference) (OtherBodyIndex :type Integer))
  (CallFunction|EndDamage))

(event OnComponentBeginOverlap(Box4)
  (params (OverlappedComponent :type Primitive%20Component%20Object%20Reference) (OtherActor :type Actor%20Object%20Reference) (OtherComp :type Primitive%20Component%20Object%20Reference) (OtherBodyIndex :type Integer) (bFromSweep :type Boolean) (SweepResult :type Hit%20Result%20Structure%20%28by%20ref%29))
  (CallFunction|StartDamage OtherActor))

(event OnComponentBeginOverlap(Box9)
  (params (OverlappedComponent :type Primitive%20Component%20Object%20Reference) (OtherActor :type Actor%20Object%20Reference) (OtherComp :type Primitive%20Component%20Object%20Reference) (OtherBodyIndex :type Integer) (bFromSweep :type Boolean) (SweepResult :type Hit%20Result%20Structure%20%28by%20ref%29))
  (CallFunction|StartDamage OtherActor))

(event OnComponentBeginOverlap(Box5)
  (params (OverlappedComponent :type Primitive%20Component%20Object%20Reference) (OtherActor :type Actor%20Object%20Reference) (OtherComp :type Primitive%20Component%20Object%20Reference) (OtherBodyIndex :type Integer) (bFromSweep :type Boolean) (SweepResult :type Hit%20Result%20Structure%20%28by%20ref%29))
  (CallFunction|StartDamage OtherActor))

(event OnComponentBeginOverlap(Box10)
  (params (OverlappedComponent :type Primitive%20Component%20Object%20Reference) (OtherActor :type Actor%20Object%20Reference) (OtherComp :type Primitive%20Component%20Object%20Reference) (OtherBodyIndex :type Integer) (bFromSweep :type Boolean) (SweepResult :type Hit%20Result%20Structure%20%28by%20ref%29))
  (CallFunction|StartDamage OtherActor))

(event OnComponentEndOverlap(Box5)
  (params (OverlappedComponent :type Primitive%20Component%20Object%20Reference) (OtherActor :type Actor%20Object%20Reference) (OtherComp :type Primitive%20Component%20Object%20Reference) (OtherBodyIndex :type Integer))
  (CallFunction|EndDamage))

(event OnComponentEndOverlap(Box10)
  (params (OverlappedComponent :type Primitive%20Component%20Object%20Reference) (OtherActor :type Actor%20Object%20Reference) (OtherComp :type Primitive%20Component%20Object%20Reference) (OtherBodyIndex :type Integer))
  (CallFunction|EndDamage))

(event Custom|Start%20Damage
  (params (Actor :type Actor%20Object%20Reference))
  (bind _returnvalue (Utilities|Time|SetTimerbyEvent (delegate Custom|DamagePlayer) 0.1 true)))

(event Custom|DamagePlayer
  (Utilities|IsValid (stale Custom|Start%20Damage Actor)
    (:Is%20Valid
      (Game|Damage|ApplyDamage (stale Custom|Start%20Damage Actor) 1.0 0 0))))

(event Custom|EndDamage
  (if (Utilities|Time|IsValidTimerHandle (stale Custom|Start%20Damage _returnvalue))
    (Utilities|Time|ClearandInvalidateTimerbyHandle (stale Custom|Start%20Damage _returnvalue))))

(event EventBeginPlay
  (CallFunction|InitializeWarningPhase)
  (Utilities|FlowControl|Delay 1.5)
  (CallFunction|InitializeAttackPhase)
  (for _array_element (Variables|Default|GetEndPos)
    (bind _returnvalue (Niagara|SpawnSystematLocation "/Game/Lightning_Electricity_Pack/Particles/P_Laser.P_Laser" (Transformation|GetActorLocation)))
    (Niagara|SetNiagaraVariable(Vector3) _returnvalue "EndPosi" (+ (Transformation|GetActorLocation) (* _array_element 5e+03))))
  (Utilities|FlowControl|Delay 5.0)
  (Actor|DestroyActor)
  (if (Utilities|Time|IsValidTimerHandle (stale Custom|Start%20Damage _returnvalue))
    (Utilities|Time|ClearandInvalidateTimerbyHandle (stale Custom|Start%20Damage _returnvalue))))

(fn ConstructionScript)

(fn InitializeWarningPhase
  (for _array_element (Utilities|Array|MakeArray (Variables|Default|GetBox5) (Variables|Default|GetBox9) (Variables|Default|GetBox4) (Variables|Default|GetBox10))
    (Collision|SetCollisionEnabled _array_element "NoCollision"))
  (for _array_element_2 (Utilities|Array|MakeArray (Variables|Default|GetCylinder1) (Variables|Default|GetCylinder2) (Variables|Default|GetCylinder3) (Variables|Default|GetCylinder))
    (Rendering|SetVisibility _array_element_2 true false)))

(fn InitializeAttackPhase
  (for _array_element (Utilities|Array|MakeArray (Variables|Default|GetBox5) (Variables|Default|GetBox9) (Variables|Default|GetBox4) (Variables|Default|GetBox10))
    (Collision|SetCollisionEnabled _array_element "QueryAndPhysics"))
  (for _array_element_2 (Utilities|Array|MakeArray (Variables|Default|GetCylinder1) (Variables|Default|GetCylinder2) (Variables|Default|GetCylinder3) (Variables|Default|GetCylinder))
    (Rendering|SetVisibility _array_element_2 false false)))