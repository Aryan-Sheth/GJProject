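; BP_Crystal is a world pickup that plays a short collection sequence when the third-person character overlaps its detection box.
; The overlap locks the character's movement, then one timeline shrinks the crystal and a second pulls it to just in front of the player.
; Both timelines lerp from the current transform each update.
; A charged energy blast Niagara effect then spawns, and after a delay movement unlocks and the crystal destroys itself.
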(event OnComponentBeginOverlap(PlayerDetectBox)
  (params (OverlappedComponent :type Primitive%20Component%20Object%20Reference) (OtherActor :type Actor%20Object%20Reference) (OtherComp :type Primitive%20Component%20Object%20Reference) (OtherBodyIndex :type Integer) (bFromSweep :type Boolean) (SweepResult :type Hit%20Result%20Structure%20%28by%20ref%29))
  (bind _returnvalue (Game|GetPlayerCharacter 0))
  (bind _returnvalue_2 (Transformation|GetActorLocation))
  (bind _asbp_third_person_character (Utilities|Casting|CastToBP_ThirdPersonCharacter OtherActor))
  (Variables|/Game/ThirdPerson/Blueprints/BP_ThirdPersonCharacter.BP_ThirdPersonCharacter_C|SetMovementLock _asbp_third_person_character true)
  (bind _rotatealpha (Timeline|RotationTimeline Play)
    (:Update
      (Transformation|SetActorScale3D (Math|Vector|Lerp(Vector) (Transformation|GetActorScale3D) "0.250000,0.250000,0.250000" _rotatealpha)))
    (:Finished
      (bind _rotatealpha_2 (Timeline|Timeline Play)
        (:Update
          (Transformation|SetActorLocation (Math|Vector|Lerp(Vector) _returnvalue_2 (+ (* (Transformation|GetActorForwardVector _returnvalue) 1e+02) (Transformation|GetActorLocation _returnvalue)) _rotatealpha_2) false false))
        (:Finished
          (Niagara|SpawnSystematLocation "/Game/MegaMagicVFXBundle/VFX/MagicalExplosionsVFX/VFX/EnergyBlast/Systems/N_EnergyBlastCharged.N_EnergyBlastCharged" _returnvalue_2)
          (Utilities|FlowControl|Delay 2.0)
          (Variables|/Game/ThirdPerson/Blueprints/BP_ThirdPersonCharacter.BP_ThirdPersonCharacter_C|SetMovementLock _asbp_third_person_character false)
          (Actor|DestroyActor))))))

(event EventBeginPlay)

(fn ConstructionScript)