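; BP_EnemySpawnManager spawns Fey and Golem enemies near the player through two custom events.
; Each picks a random reachable point within a radius of the player and plays a spawn particle effect there.
; After delays it spawns the character, deactivates the effect, then starts the Fey's AI or the Golem's intro sequence.
; The Golem spawn adds riser and explosion sounds, a longer wait and an enlarged scale.
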(event Custom|SpawnGolem
  (bind _output_get (Variables|Default|SetRandom%20Location (.RandomLocation (AI|Navigation|GetRandomReachablePointinRadius (Transformation|GetActorLocation (Game|GetPlayerCharacter 0)) 2e+03 0 0))))
  (Audio|PlaySound2D "/Game/Game/SFX/SciFiRiser.SciFiRiser" 1.0 1.0 0.0 0 0)
  (bind _returnvalue (Niagara|SpawnSystematLocation "/Game/MsvFx_Niagara_SlashFx_Pack/Prefabs/P_Spawn_Energy_Light.P_Spawn_Energy_Light" _output_get "0, 0, 0" "7.000000,7.000000,7.000000"))
  (Utilities|FlowControl|Delay 5.0)
  (bind _returnvalue_2 (Game|SpawnActorfromClass "/Game/Game/Blueprints/Enemies/BP_Golem.BP_Golem_C" (Math|Transform|MakeTransform (Variables|Default|GetRandom%20Location) "0, 0, 0" "7.000000,7.000000,7.000000") "AdjustIfPossibleButAlwaysSpawn" "MultiplyWithRoot" 0 0))
  (Utilities|FlowControl|Delay 1.0)
  (Audio|PlaySound2D "/Game/Game/SFX/SiFiExplosion.SiFiExplosion" 1.0 1.0 0.0 0 0)
  (Components|Activation|Deactivate _returnvalue)
  (Default|PlayStartSequence _returnvalue_2))

(event Custom|SpawnNature
  (bind _output_get (Variables|Default|SetRandom%20Location (.RandomLocation (AI|Navigation|GetRandomReachablePointinRadius (Transformation|GetActorLocation (Game|GetPlayerCharacter 0)) 2e+03 0 0))))
  (bind _returnvalue (Niagara|SpawnSystematLocation "/Game/MsvFx_Niagara_SlashFx_Pack/Prefabs/P_Spawn_Energy_Nature.P_Spawn_Energy_Nature" _output_get "0, 0, 0" "7.000000,7.000000,7.000000"))
  (Utilities|FlowControl|Delay 2.0)
  (bind _returnvalue_2 (Game|SpawnActorfromClass "/Game/Game/Blueprints/Enemies/FeyPlayerCharacter.FeyPlayerCharacter_C" (Math|Transform|MakeTransform (Variables|Default|GetRandom%20Location) "0, 0, 0" "1.000000,1.000000,1.000000") "AdjustIfPossibleButAlwaysSpawn" "MultiplyWithRoot" 0 0))
  (Utilities|FlowControl|Delay 1.0)
  (Components|Activation|Deactivate _returnvalue)
  (Default|StartAI _returnvalue_2))

(event EventBeginPlay)

(fn ConstructionScript)