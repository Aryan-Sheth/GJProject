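; World progression manager that drives the game's story beats, from crystal and skill tutorial through the Light and Nature boss stages.
; Bound defeat events and externally called milestone events spawn a guiding fairy behind the player to play numbered dialogue, often after a delay.
; Spawn events place the crystal behind the player or tell BP_EnemySpawnManager to spawn the Golem or Nature encounter.
; A helper crossfades the tracked background music between stages.
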(event Custom|SpawnLight
  (Utilities|FlowControl|Sequence
    (:then_0
      (Utilities|CrossFadeAudioinDuration "/Game/Game/SFX/Distant-Sky-Epic-Hybrid-Music-chosic_com_.Distant-Sky-Epic-Hybrid-Music-chosic_com_" 3.0))
    (:then_1
      (bind _returnvalue (Actor|GetActorOfClass "/Game/Game/Blueprints/World/BP_EnemySpawnManager.BP_EnemySpawnManager_C"))
      (Default|SpawnGolem _returnvalue)
      (Default|CallLightSpawned))))

(event Custom|SpawnNature
  (Utilities|FlowControl|Sequence
    (:then_0
      (Utilities|CrossFadeAudioinDuration "/Game/Game/SFX/yoitrax-warrior_chosic_com_.yoitrax-warrior_chosic_com_" 5.0))
    (:then_1
      (bind _returnvalue (Actor|GetActorOfClass "/Game/Game/Blueprints/World/BP_EnemySpawnManager.BP_EnemySpawnManager_C"))
      (Default|SpawnNature _returnvalue))))

(event Custom|LightDefeated_Event
  (Utilities|CrossFadeAudioinDuration "/Game/Game/SFX/DaylightCue.DaylightCue" 3.0)
  (Utilities|FlowControl|Delay 5.0)
  (CallFunction|SpawnFairyandPlayDialogue 2))

(event Custom|WorldDefeated_Event
  (Utilities|CrossFadeAudioinDuration "/Game/Game/SFX/Memories-of-Spring_chosic_com_.Memories-of-Spring_chosic_com_" 5.0)
  (Utilities|FlowControl|Delay 3e+01)
  (CallFunction|SpawnFairyandPlayDialogue 4))

(event Custom|SpawnCrystal
  (bind _returnvalue (Game|Player|GetPlayerPawn 0))
  (Game|SpawnActorfromClass "/Game/Game/Blueprints/World/BP_Crystal.BP_Crystal_C" (Math|Transform|MakeTransform (+ (Transformation|GetActorLocation _returnvalue) (* (Transformation|GetActorForwardVector _returnvalue) 1.5e+03 -1.0)) "0, 0, 0" "1.000000,1.000000,1.000000") "AdjustIfPossibleButAlwaysSpawn" "MultiplyWithRoot" 0 0))

(event Custom|CrystalTouched
  (CallFunction|SpawnFairyandPlayDialogue 1))

(event Custom|SkillTutorialComplete
  (Utilities|FlowControl|Delay 5.0)
  (CallFunction|SpawnFairyandPlayDialogue 3))

(event EventBeginPlay
  (bind _returnvalue (Audio|SpawnSound2D "/Game/Game/SFX/sci-fi-survival-dreamscape-6319.sci-fi-survival-dreamscape-6319" 1.0 1.0 0.0 0))
  (Variables|Default|SetCurrentBGM _returnvalue)
  (Utilities|FlowControl|Delay 15.0)
  (CallFunction|SpawnFairyandPlayDialogue)
  (EventDispatchers|BindEventtoLightDefeated (delegate Custom|LightDefeated_Event))
  (EventDispatchers|BindEventtoWorldDefeated (delegate Custom|WorldDefeated_Event)))

(fn ConstructionScript)

(fn SpawnFairyandPlayDialogue
  (params (DialogueNum :type Integer))
  (bind _returnvalue (Game|GetPlayerCharacter 0))
  (bind _returnvalue_2 (Game|SpawnActorfromClass "/Game/Game/Blueprints/AI/Fairy/BP_GuidingFairy.BP_GuidingFairy_C" (Math|Transform|MakeTransform (+ (Transformation|GetActorLocation _returnvalue) (* (Transformation|GetActorForwardVector _returnvalue) 1e+03 -1.0)) "0, 0, 0" "1.000000,1.000000,1.000000") "Undefined" "MultiplyWithRoot" 0 0))
  (Default|PlayDialogue _returnvalue_2 DialogueNum))